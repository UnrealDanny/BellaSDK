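; BP_Valve is an interactable valve that turns one full revolution and notifies another actor.
; Interaction calls ValveMove and sends a message to the referenced Actor.
; A Timeline drives the Cube's pitch, playing forward or reversing from the end according to ValveMoving.
; A FlipFlop on Timeline completion toggles that flag, and a DoOnce blocks repeated reversals until the return turn finishes.
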(event `ValveMove`
  (if (not (`self.ValveMoving?`))
    (bind (_direction _newtrack_0) (`Timeline|Timeline` :!label _label)
      (:`Update`
        (`SceneComponent.K2_SetRelativeRotation` (`self.Cube`) (`KismetMathLibrary.MakeRotator` 0.0 (`KismetMathLibrary.Lerp` 0.0 -360.0 _newtrack_0)) false false))
      (:`Finished`
        (`/Engine/EditorBlueprintResources/StandardMacros.FlipFlop`
          (:`A`
            (set `self.ValveMoving?` true))
          (:`B`
            (set `self.ValveMoving?` false)
            (`self.Finished`)))))
    (else
      (`/Engine/EditorBlueprintResources/StandardMacros.DoOnce` false :!label _label_2
        (:`Completed`
          (goto _label :!via `ReverseFromEnd`))))))

(event `Finished`
  (goto _label_2 :!via `Reset`))

(event `/Game/BlueprintsTest/Interfaces/BPI_Interaction.Interaction`
  ; Interaction
  (if (`self.DoOnce?`)
    (`/Engine/EditorBlueprintResources/StandardMacros.DoOnce` false
      (:`Completed`
        _)))
  (`self.ValveMove`)
  (message `/Game/BlueprintsTest/Interfaces/BPI_Communicator.SendMessage` (`self.Actor`)))

(fn `UserConstructionScript`)