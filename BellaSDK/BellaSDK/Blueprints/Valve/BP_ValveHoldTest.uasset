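; BP_ValveHoldTest is a test actor for a hold-type valve that moves a cube like a gate.
; BeginPlay binds an event to the valve's active notification, and MovingGate takes a Holding flag.
; Holding plays a timeline that lerps the cube upward, while releasing reverses it at double speed.
; A separate SendMessage event switches on a point light.
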(event `/Game/BlueprintsTest/Interfaces/BPI_Communicator.SendMessage`
  (`SceneComponent.SetVisibility` (`self.PointLight`) true false))

(event `self.ReceiveBeginPlay`
  (add `/Game/Blueprints/Valve/BP_ValveHold.ValveActive` (`self.Valve`) (`|CreateDelegate` :!event `MovingGate`)))

(event `MovingGate`
  (params (`Holding?` :type Boolean))
  (if `Holding?`
    (`TimelineComponent.SetPlayRate` (`self.Timeline`) 1.0)
    (bind (_direction _newtrack_0) (`Timeline|Timeline` :!label _label)
      (:`Update`
        (`SceneComponent.K2_SetRelativeLocation` (`self.Cube`) (`KismetMathLibrary.MakeVector` 0.0 0.0 (`KismetMathLibrary.Lerp` 0.0 500.0 _newtrack_0)) false false)))
    (else
      (`TimelineComponent.SetPlayRate` (`self.Timeline`) 2.0)
      (goto _label :!via `Reverse`))))

(fn `UserConstructionScript`)