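; A hold-to-turn valve interactable that messages a linked Actor once fully turned.
; Holding plays a timeline that pitches the Cube and signals the valve active; releasing early signals inactive and reverses at double speed.
; At full rotation it sets Finished and uses a DoOnce to play a shutter sound and send the message.
; Releasing after completion skips the rewind and resets the DoOnce after a short delay.
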(event `/Game/BlueprintsTest/Interfaces/BPI_InteractHold.InteractHold`
  (params (`Holding?` :type Boolean))
  (if `Holding?`
    (`TimelineComponent.SetPlayRate` (`self.TimelineRotate`) 1.0)
    (`self.ValveActive` true)
    (bind (_direction _rotationspeed) (`Timeline|TimelineRotate` :`NewTime` 1.0 :!label _label)
      (:`Update`
        (`SceneComponent.K2_SetRelativeRotation` (`self.Cube`) (`KismetMathLibrary.MakeRotator` 0.0 (`KismetMathLibrary.Lerp` 0.0 500.0 _rotationspeed)) false false)
        (if (== _rotationspeed 1.0)
          (set `self.Finished` true)
          (`/Engine/EditorBlueprintResources/StandardMacros.DoOnce` false :!label _label_2
            (:`Completed`
              (`GameplayStatics.PlaySoundAtLocation` "/Engine/VREditor/Sounds/UI/Camera_Shutter.Camera_Shutter" (`self.K2_GetActorLocation`) (struct) 1.0 1.0 0.0 null null null null)
              (message `/Game/BlueprintsTest/Interfaces/BPI_Communicator.SendMessage` (`self.Actor`)))))))
    (elif (not (`self.Finished`))
      (`TimelineComponent.SetPlayRate` (`self.TimelineRotate`) 2.0)
      (`self.ValveActive` false)
      (goto _label :!via `Reverse`)
      (else
        (`KismetSystemLibrary.Delay` 0.2)
        (goto _label_2 :!via `Reset`)))))

(fn `UserConstructionScript`)