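; BP_DoorInteract is an interactable door that alternates between opening and closing on each Interaction event, ignored while its timeline is playing.
; When opening, SetDoorOpenAngle uses a dot product of the actor's forward vector and direction to the passed location to choose a positive or negative 90-degree swing by side.
; The timeline lerps scene component yaw in world space and reverses to close.
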(event `/Game/BlueprintsTest/Interfaces/BPI_Interaction.Interaction`
  (params (Location :type "Vector Structure"))
  (if (not (`TimelineComponent.IsPlaying` (`self.TL_Door`)))
    (`/Engine/EditorBlueprintResources/StandardMacros.FlipFlop`
      (:`A`
        (`self.SetDoorOpenAngle` Location)
        (bind (_direction _alpha) (`Timeline|TL_Door` :!label _label)
          (:`Update`
            (`SceneComponent.K2_SetWorldRotation` (`self.Scene`) (`KismetMathLibrary.MakeRotator` 0.0 0.0 (`KismetMathLibrary.Lerp` 0.0 (`self.DoorOpenAngle`) _alpha)) false false)
            (`SceneComponent.K2_SetWorldRotation` (`self.Scene`) (`KismetMathLibrary.MakeRotator` 0.0 0.0 (`KismetMathLibrary.Lerp` 0.0 (`self.DoorOpenAngle`) _alpha)) false false))))
      (:`B`
        (goto _label :!via `Reverse`)))))

(fn `SetDoorOpenAngle`
  (params (PlayerLocation :type "Vector Structure"))
  (set `self.DoorOpenAngle` (`KismetMathLibrary.SelectFloat` -90.0 90.0 (>= (`KismetMathLibrary.Dot_VectorVector` (`KismetMathLibrary.GetDirectionUnitVector` (`self.K2_GetActorLocation`) (`local.PlayerLocation`)) (`self.GetActorForwardVector`)) 0.0)))
  (return))

(fn `UserConstructionScript`)