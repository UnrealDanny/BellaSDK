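; BP_LightSwitch is an interactable light switch that flips between two states and messages a referenced Actor.
; Interaction calls ToggleSwitch, then SendMessageMessage on that Actor, with a DoOnce check at the start.
; ToggleSwitch inverts IsON, tilts the Switch component to opposite pitch angles and prints debug text that reads opposite to the new IsON value.
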(event `ToggleSwitch`
  (bind _switch (`self.Switch`))
  (if (`self.IsON?`)
    (set `self.IsON?` false)
    (`KismetSystemLibrary.PrintString` "ON")
    (`SceneComponent.K2_SetRelativeRotation` _switch (struct :`Roll` 10.0) false false)
    (else
      (set `self.IsON?` true)
      (`KismetSystemLibrary.PrintString` "OFF" true true (struct :`G` 0.66 :`B` 1.0 :`A` 1.0) 4.0)
      (`SceneComponent.K2_SetRelativeRotation` _switch (struct :`Roll` -10.0) false false))))

(event `/Game/BlueprintsTest/Interfaces/BPI_Interaction.Interaction`
  (if (`self.DoOnce?`)
    (`/Engine/EditorBlueprintResources/StandardMacros.DoOnce` false
      (:`Completed`
        _)))
  (`self.ToggleSwitch`)
  (message `/Game/BlueprintsTest/Interfaces/BPI_Communicator.SendMessage` (`self.Actor`)))

(fn `UserConstructionScript`)