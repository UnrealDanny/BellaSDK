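; BP_DoorNKey is a locked door actor that opens once enough keys are collected.
; Each SendMessage call increments the key count and sets GotKey when the count exactly equals the required number.
; Interaction either calls OpenDoor, which destroys the actor, or prints that it is locked.
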(event `OpenDoor`
  (`self.K2_DestroyActor`))

(event `/Game/BlueprintsTest/Interfaces/BPI_Interaction.Interaction`
  (params (Location :type "Vector Structure"))
  (if (stale `/Game/BlueprintsTest/Interfaces/BPI_Communicator.SendMessage` _output_get_2)
    (`self.OpenDoor`)
    (`KismetSystemLibrary.PrintString` "OPENED!")
    (else
      (`KismetSystemLibrary.PrintString` "Locked!"))))

(event `/Game/BlueprintsTest/Interfaces/BPI_Communicator.SendMessage`
  (bind _result (`/Engine/EditorBlueprintResources/StandardMacros.IncrementInt` (`self.NumOfKeys`))
    (:`  `
      (bind _output_get (set `self.NumOfKeys` _result))
      (bind _output_get_2 (set `self.GotKey?` (== _output_get (`self.NecessaryNumOfKeys`)))))))

(fn `UserConstructionScript`)