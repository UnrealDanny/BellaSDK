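; BP_LeverTestBox is a test Blueprint with a cube that shows or hides when it receives a SendMessage event, apparently as a target for the wall lever.
; SendMessage calls ToggleCubeVisibility, which flips the IsVisible flag and sets the Cube component's visibility to match, without propagating to children.
; Each toggle prints the new state as a debug string.
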(event `ToggleCubeVisibility`
  (bind _cube (`self.Cube`))
  (if (`self.IsVisible?`)
    (set `self.IsVisible?` false)
    (`SceneComponent.SetVisibility` _cube false false)
    (`KismetSystemLibrary.PrintString` "NOT VISIBLE")
    (else
      (set `self.IsVisible?` true)
      (`SceneComponent.SetVisibility` _cube true false)
      (`KismetSystemLibrary.PrintString` " VISIBLE"))))

(event `/Game/BlueprintsTest/Interfaces/BPI_Communicator.SendMessage`
  (`self.ToggleCubeVisibility`))

(fn `UserConstructionScript`)