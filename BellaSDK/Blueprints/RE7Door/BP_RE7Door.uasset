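; Interactable door Blueprint, named after RE7, that cycles through closed, partly open and fully open with each interaction, swinging away from or toward closed.
; Each interaction picks a target yaw from the current state, signed by the camera's facing relative to an Arrow component.
; A looping timer rotates the door scene component toward that angle at constant speed.
; Tick derives the state from the current yaw.
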(event `self.ReceiveTick`
  (params (DeltaSeconds :type "Float (single-precision)"))
  (`self.SetDoorState`))

(event `/Game/BlueprintsTest/Interfaces/BPI_Interaction.Interaction`
  (switch `/Game/BlueprintsTest/RE7Door/E_DoorState` (`self.DoorState`)
    (:`NewEnumerator0`
      (bind _sidedoor (`self.DoorSide`))
      (bind _output_get (set `self.TargetAngle` 15.0))
      (set `self.TargetAngle` (* _output_get _sidedoor))
      (`self.StartInteractingDoor`))
    (:`NewEnumerator1`
      (bind _sidedoor_2 (`self.DoorSide`))
      (bind _output_get_2 (set `self.TargetAngle` 90.0))
      (set `self.TargetAngle` (* _output_get_2 _sidedoor_2))
      (`self.StartInteractingDoor`))
    (:`NewEnumerator2`
      (`self.DoorSide`)
      (set `self.TargetAngle` 0.0)
      (`self.StartInteractingDoor`))))

(event `StartInteractingDoor`
  (`KismetSystemLibrary.K2_SetTimerDelegate` (delegate `CustomEvent`) 0.01 true))

(event `CustomEvent`
  (`SceneComponent.K2_SetRelativeRotation` (`self.DoorScene`) (`KismetMathLibrary.MakeRotator` 0.0 0.0 (`KismetMathLibrary.FInterpTo_Constant` (.yaw (`SceneComponent.RelativeRotation` (`self.DoorScene`))) (`self.TargetAngle`) (`GameplayStatics.GetWorldDeltaSeconds`) (`self.Interp Speed`))) false false))

(fn `DoorSide`
  (returns (SideDoor :type "Float (double-precision)"))
  (if (< (`KismetMathLibrary.Dot_VectorVector` (`KismetMathLibrary.GetForwardVector` (`PlayerCameraManager.GetCameraRotation` (`GameplayStatics.GetPlayerCameraManager` 0))) (`SceneComponent.GetForwardVector` (`self.Arrow`))) 0.0)
    (bind _output_get (set `self.SideDoor` -1.0))
    (return _output_get)
    (else
      (bind _output_get_2 (set `self.SideDoor` 1.0))
      (return _output_get_2))))

(fn `SetDoorState`
  (bind (_relativerotation_roll _relativerotation_pitch _relativerotation_yaw) (`KismetMathLibrary.BreakRotator` (`SceneComponent.RelativeRotation` (`self.DoorScene`))))
  (if (or (and (>= _relativerotation_yaw 0.0) (< _relativerotation_yaw 1.0)) (and (<= _relativerotation_yaw 0.0) (> _relativerotation_yaw -1.0)))
    (set `self.DoorState` "NewEnumerator0")
    (elif (or (and (> _relativerotation_yaw 1.0) (< _relativerotation_yaw 89.0)) (and (< _relativerotation_yaw -1.0) (> _relativerotation_yaw -89.0)))
      (set `self.DoorState` "NewEnumerator1")
      (elif (or (and (> _relativerotation_yaw 89.0) (< _relativerotation_yaw 91.0)) (and (< _relativerotation_yaw -89.0) (> _relativerotation_yaw -91.0)))
        (set `self.DoorState` "NewEnumerator2")))))

(fn `UserConstructionScript`)