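; BP_FlickerLight is a spotlight actor that can be toggled and flickers between two intensities.
; ToggleLight, also called by SendMessage, flips IsON and shows or hides the SpotLight, with the true branch showing it.
; Showing it starts an endless RetriggerableDelay and FlipFlop loop that alternates MinIntensity and Intensity at random intervals, with no stop on hide.
; The construction script applies the base Intensity.
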(event `ToggleLight`
  (bind _spotlight (`self.SpotLight`))
  (if (`self.IsON?`)
    (set `self.IsON?` false)
    (`SceneComponent.SetVisibility` _spotlight true false)
    (`KismetSystemLibrary.RetriggerableDelay` (`KismetMathLibrary.RandomFloatInRange` (`self.Min`) (`self.Max`)) :!label _label)
    (`/Engine/EditorBlueprintResources/StandardMacros.FlipFlop`
      (:`A`
        (`LightComponent.SetIntensity` (`self.SpotLight`) (`self.MinIntensity`))
        (goto _label))
      (:`B`
        (`LightComponent.SetIntensity` (`self.SpotLight`) (`self.Intensity`))
        (goto _label)))
    (else
      (set `self.IsON?` true)
      (`SceneComponent.SetVisibility` _spotlight false false))))

(event `/Game/BlueprintsTest/Interfaces/BPI_Communicator.SendMessage`
  (`self.ToggleLight`))

(fn `UserConstructionScript`
  (`LightComponent.SetIntensity` (`self.SpotLight`) (`self.Intensity`)))