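; Interactable wall lever that rotates its Scene component around the roll axis and messages a referenced Actor when used.
; Interaction calls ToggleLever, then sends the message to that Actor.
; A DoOnce boolean picks the motion: when set, a FlipFlop only plays a separate timeline with no reverse.
; Otherwise, a FlipFlop alternately plays and reverses the main timeline to swing the lever back and forth.
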(event `ToggleLever`
  (if (`self.DoOnce?`)
    (`/Engine/EditorBlueprintResources/StandardMacros.FlipFlop`
      (:`A`
        (bind (_direction _newtrack_0) (`Timeline|Timeline_0`)
          (:`Update`
            (`SceneComponent.K2_SetRelativeRotation` (`self.Scene`) (`KismetMathLibrary.MakeRotator` _newtrack_0) false false)))))
    (else
      (`/Engine/EditorBlueprintResources/StandardMacros.FlipFlop`
        (:`A`
          (bind (_direction_2 _newtrack_0_2) (`Timeline|Timeline` :!label _label)
            (:`Update`
              (`SceneComponent.K2_SetRelativeRotation` (`self.Scene`) (`KismetMathLibrary.MakeRotator` _newtrack_0_2) false false))))
        (:`B`
          (goto _label :!via `Reverse`))))))

(event `/Game/BlueprintsTest/Interfaces/BPI_Interaction.Interaction`
  (if (`self.DoOnce?`)
    (`/Engine/EditorBlueprintResources/StandardMacros.DoOnce` false
      (:`Completed`
        _)))
  (`self.ToggleLever`)
  (message `/Game/BlueprintsTest/Interfaces/BPI_Communicator.SendMessage` (`self.Actor`)))

(fn `UserConstructionScript`)