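; BP_PressureGate is a gate that rises once the required number of linked pressure plates is active.
; On BeginPlay it binds to the plates' activation dispatchers, but only if the Trigger array's length matches the required count.
; Each plate signal adjusts and prints a running counter.
; Reaching the target plays a timeline that lerps the gate's relative Z, while any deactivation reverses it.
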(event `GateOn/Off`
  (params (`IsActive?` :type Boolean))
  (if `IsActive?`
    (bind _result (`/Engine/EditorBlueprintResources/StandardMacros.IncrementInt` (`self.PressureSwitchesActivated`))
      (:`  `
        (bind _output_get (set `self.PressureSwitchesActivated` _result))
        (`KismetSystemLibrary.PrintString` (`KismetStringLibrary.Conv_IntToString` _output_get))
        (if (== (`self.PressureSwitchesNeeded`) (`self.PressureSwitchesActivated`))
          (bind (_direction _doorposition) (`Timeline|DoorActivation` :!label _label)
            (:`Update`
              (`SceneComponent.K2_SetRelativeLocation` (`self.Gate`) (`KismetMathLibrary.MakeVector` 0.0 0.0 (`KismetMathLibrary.Lerp` 250.0 500.0 _doorposition)) false false))))))
    (else
      (bind _result_2 (`/Engine/EditorBlueprintResources/StandardMacros.DecrementInt` (`self.PressureSwitchesActivated`))
        (:`  `
          (bind _output_get_2 (set `self.PressureSwitchesActivated` _result_2))
          (`KismetSystemLibrary.PrintString` (`KismetStringLibrary.Conv_IntToString` _output_get_2))
          (goto _label :!via `Reverse`))))))

(event `self.ReceiveBeginPlay`
  (if (== (`KismetArrayLibrary.Array_Length` (`self.Trigger`)) (`self.PressureSwitchesNeeded`))
    (add `/Game/Blueprints/PressurePlate/BP_PressurePlate.OnPlateActivated` (`self.Trigger`) (`|CreateDelegate` :!event `GateOn/Off`))))

(fn `UserConstructionScript`)