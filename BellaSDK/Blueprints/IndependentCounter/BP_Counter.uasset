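; BP_Counter is a counter Blueprint that ends the game with a win once a target number of triggers is reached.
; Each Message event increments TriggerNumber and prints the count.
; When the count equals MaxNumber, it prints a win message, pauses the game, adds a WBP_HUD widget to the viewport and shows the mouse cursor.
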(event `/Game/Blueprints/BPI_Communicator.Message`
  (bind _result (`/Engine/EditorBlueprintResources/StandardMacros.IncrementInt` (`self.TriggerNumber`))
    (:`  `
      (`KismetSystemLibrary.PrintString` (`KismetStringLibrary.Conv_IntToString` _result))
      (if (== (`self.TriggerNumber`) (`self.MaxNumber`))
        (`KismetSystemLibrary.PrintString` "You Won!")
        (`GameplayStatics.SetGamePaused` true)
        (bind _returnvalue (`|CreateWidget` "/Game/Blueprints/WBP_HUD.WBP_HUD_C"))
        (`UserWidget.AddToViewport` _returnvalue 0)
        (set `PlayerController.bShowMouseCursor` true (`GameplayStatics.GetPlayerController` 0))))))

(fn `UserConstructionScript`)