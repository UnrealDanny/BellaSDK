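; BP_ButtonPlatform is an interactable button that raises and lowers a BP_Platform found in the level by class lookup.
; On Interaction, a FlipFlop alternately plays and reverses a Timeline that lerps the relative height of the button's Sphere and the platform's Cube together.
; A Moving flag ignores further presses until the Timeline finishes and a short delay elapses.
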(event `/Game/BlueprintsTest/Interfaces/BPI_Interaction.Interaction`
  (if (not (`self.Moving?`))
    (set `self.Moving?` true)
    (bind _returnvalue (`GameplayStatics.GetActorOfClass` "/Game/Blueprints/Platform/BP_Platform.BP_Platform_C"))
    (`/Engine/EditorBlueprintResources/StandardMacros.FlipFlop`
      (:`A`
        (bind (_direction _newtrack_0) (`Timeline|Timeline` :!label _label)
          (:`Update`
            (`SceneComponent.K2_SetRelativeLocation` (`self.Sphere`) (`KismetMathLibrary.MakeVector` 0.0 0.0 (`KismetMathLibrary.Lerp` 0.0 400.0 _newtrack_0)) false false)
            (`SceneComponent.K2_SetRelativeLocation` (`/Game/Blueprints/Platform/BP_Platform.Cube` _returnvalue) (`KismetMathLibrary.MakeVector` 0.0 0.0 (`KismetMathLibrary.Lerp` 0.0 400.0 _newtrack_0)) false false))
          (:`Finished`
            (`KismetSystemLibrary.Delay` 0.5)
            (set `self.Moving?` false))))
      (:`B`
        (goto _label :!via `Reverse`)))))

(fn `UserConstructionScript`)