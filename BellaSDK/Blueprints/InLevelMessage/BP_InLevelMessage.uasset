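; BP_InLevelMessage is an in-level message marker that displays a UI widget while something overlaps its Sphere trigger.
; Overlap begin hides the Cube and adds a widget of the configured Class to the viewport, without filtering the overlapping actor.
; Overlap end removes the widget, reveals the Cube, and gives it a new M_ILM_Green dynamic material instance with its Color parameter set to white.
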(event `self.Sphere.OnComponentBeginOverlap`
  (params (OverlappedComponent :type "PrimitiveComponent Object Reference") (OtherActor :type "Actor Object Reference") (OtherComp :type "PrimitiveComponent Object Reference") (OtherBodyIndex :type Integer) (bFromSweep :type Boolean) (SweepResult :type "HitResult Structure (by ref)"))
  (`SceneComponent.SetHiddenInGame` (`self.Cube`) true false)
  (bind _returnvalue (`|CreateWidget` (`self.Class`)))
  (`UserWidget.AddToViewport` _returnvalue 0))

(event `self.Sphere.OnComponentEndOverlap`
  (params (OverlappedComponent :type "PrimitiveComponent Object Reference") (OtherActor :type "Actor Object Reference") (OtherComp :type "PrimitiveComponent Object Reference") (OtherBodyIndex :type Integer))
  (`SceneComponent.SetHiddenInGame` (`self.Cube`) false false)
  (`Widget.RemoveFromParent` (stale `self.Sphere.OnComponentBeginOverlap` _returnvalue))
  (bind _returnvalue (`PrimitiveComponent.CreateDynamicMaterialInstance` (`self.Cube`) 0 "/Game/Blueprints/InLevelMessage/M_ILM_Green.M_ILM_Green" "None"))
  (`MaterialInstanceDynamic.SetVectorParameterValue` _returnvalue "Color" (make `LinearColor` 1.0 1.0 1.0 1.0)))

(fn `UserConstructionScript`)