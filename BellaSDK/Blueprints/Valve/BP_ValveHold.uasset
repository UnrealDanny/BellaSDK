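; BP_ValveHold is a valve that turns through repeated Interaction calls and unwinds when they stop.
; A call counter plays a Timeline from the second call onward, lerping the Cube's pitch.
; The first call starts a short retriggerable delay that resets the counter and reverses the Timeline if unfinished.
; Reaching the end of the track sets Finished, which blocks further interaction.
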(event `/Game/BlueprintsTest/Interfaces/BPI_Interaction.Interaction`
  (params (Location :type "Vector Structure"))
  (if (not (`self.Finished`))
    (bind _result (`/Engine/EditorBlueprintResources/StandardMacros.IncrementInt` (`self.NumOfCalls`))
      (:`  `
        (set `self.NumOfCalls` _result)
        (if (> (`self.NumOfCalls`) 1)
          (bind (_direction _newtrack_0) (`Timeline|Timeline` :!label _label)
            (:`Update`
              (`SceneComponent.K2_SetRelativeRotation` (`self.Cube`) (`KismetMathLibrary.MakeRotator` 0.0 (`KismetMathLibrary.Lerp` 0.0 500.0 _newtrack_0)) false false)
              (if (>= _newtrack_0 1.0)
                (set `self.Finished` true))))
          (else
            (`KismetSystemLibrary.RetriggerableDelay` 0.2)
            (set `self.NumOfCalls` 0)
            (if (not (`self.Finished`))
              (goto _label :!via `Reverse`))))))))

(fn `UserConstructionScript`)